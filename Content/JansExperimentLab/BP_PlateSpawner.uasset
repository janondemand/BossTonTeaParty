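; BP_PlateSpawner spawns three BP_Plate actors and runs them through shielding, positioning and launching states.
; Tick rolls the Scene component during Shielding until a timer expires, then PositionPlates detaches the plates and snapshots source and target transforms.
; Positioning uses timed lerps on plate transforms, though alpha runs negative and target rotations are never wired in.
; LaunchPlates only sets the Launching state, which has no behavior here.
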(event Custom|PositionPlates
  (bind _plategroup (Variables|Default|GetPlateGroup))
  (bind _plategroup_2 (Variables|Default|GetPlateGroup))
  (Variables|Default|SetPlateState "NewEnumerator1")
  (for _array_element (Variables|Default|GetPlateGroup)
    (Transformation|DetachFromActor _array_element "KeepWorld" "KeepWorld" "KeepWorld")
    (Variables|Default|SetPlateTargetLocations (Utilities|Array|MakeArray (Transformation|GetWorldLocation (Variables|Default|GetPlatePosition1)) (Transformation|GetWorldLocation (Variables|Default|GetPlatePosition2)) (Transformation|GetWorldLocation (Variables|Default|GetPlatePosition3))))
    (Variables|Default|SetPlateSourceLocations (Utilities|Array|MakeArray (Transformation|GetWorldLocation (Variables|/Script/Engine.Actor|GetRootComponent (Utilities|Array|Get(acopy) _plategroup_2))) (Transformation|GetWorldLocation (Variables|/Script/Engine.Actor|GetRootComponent (Utilities|Array|Get(acopy) _plategroup_2 1))) (Transformation|GetWorldLocation (Variables|/Script/Engine.Actor|GetRootComponent (Utilities|Array|Get(acopy) _plategroup_2 2)))))
    (Variables|Default|SetSourceRotations (Utilities|Array|MakeArray (Transformation|GetWorldRotation (Variables|/Script/Engine.Actor|GetRootComponent (Utilities|Array|Get(acopy) _plategroup))) (Transformation|GetWorldRotation (Variables|/Script/Engine.Actor|GetRootComponent (Utilities|Array|Get(acopy) _plategroup 1))) (Transformation|GetWorldRotation (Variables|/Script/Engine.Actor|GetRootComponent (Utilities|Array|Get(acopy) _plategroup 2)))))
    (Variables|Default|SetTargetRotations (Utilities|Array|MakeArray (Transformation|GetWorldRotation (Variables|Default|GetPlatePosition1)) (Transformation|GetWorldRotation (Variables|Default|GetPlatePosition2)) (Transformation|GetWorldRotation (Variables|Default|GetPlatePosition3))))
    (Variables|Default|SetPositioningStartTime (Utilities|Time|GetGameTimeinSeconds))))

(event Custom|LaunchPlates
  (Variables|Default|SetPlateState "NewEnumerator2"))

(event EventBeginPlay
  (Variables|Default|SetStartTime (Utilities|Time|GetGameTimeinSeconds))
  (bind _returnvalue (Game|SpawnActorfromClass "/Game/JansExperimentLab/BP_Plate.BP_Plate_C" (Transformation|GetWorldTransform (Variables|Default|GetPlateStart0)) "Undefined" "MultiplyWithRoot" 0 "0.000000,0.000000,0.000000" 0))
  (Utilities|Array|Add (Variables|Default|GetPlateGroup) _returnvalue)
  (bind _returnvalue_2 (Game|SpawnActorfromClass "/Game/JansExperimentLab/BP_Plate.BP_Plate_C" (Transformation|GetWorldTransform (Variables|Default|GetPlateStart1)) "Undefined" "MultiplyWithRoot" 0 "0.000000,0.000000,0.000000" 0))
  (Utilities|Array|Add (Variables|Default|GetPlateGroup) _returnvalue_2)
  (bind _returnvalue_3 (Game|SpawnActorfromClass "/Game/JansExperimentLab/BP_Plate.BP_Plate_C" (Transformation|GetWorldTransform (Variables|Default|GetPlateStart2)) "Undefined" "MultiplyWithRoot" 0 "0.000000,0.000000,0.000000" 0))
  (Utilities|Array|Add (Variables|Default|GetPlateGroup) _returnvalue_3))

(event Collision|EventActorBeginOverlap
  (params (OtherActor :type Actor%20Object%20Reference)))

(event EventTick
  (params (DeltaSeconds :type Float%20%28single-precision%29))
  (bind _returnvalue (Utilities|Time|GetGameTimeinSeconds))
  (bind _positioningstarttime (Variables|Default|GetPositioningStartTime))
  (bind _positioningduration (Variables|Default|GetPositioningDuration))
  (bind _returnvalue_2 (- _positioningstarttime _returnvalue))
  (bind _returnvalue_3 (/ _returnvalue_2 _positioningduration))
  (switch Utilities|FlowControl|Switch|SwitchonEnum_PlateState (Variables|Default|GetPlateState)
    (:NewEnumerator0
      (Transformation|AddLocalRotation (Variables|Default|GetScene) (Math|Rotator|MakeRotator (* (Variables|Default|GetRotationSpeed) (Utilities|Time|GetWorldDeltaSeconds)) 0.0 0.0) false false)
      (if (not (>= (+ (Variables|Default|GetStartTime) (Variables|Default|GetShieldDuration)) (Utilities|Time|GetGameTimeinSeconds)))
        (CallFunction|PositionPlates)))
    (:NewEnumerator1
      (for (_array_element _array_index) (Variables|Default|GetPlateGroup)
        (Transformation|SetWorldLocation (stale _array_element) (Math|Vector|Lerp(Vector) (Utilities|Array|Get(acopy) (Variables|Default|GetPlateSourceLocations) _array_index) (Utilities|Array|Get(acopy) (Variables|Default|GetPlateTargetLocations) _array_index) _returnvalue_3) false false)
        (Transformation|SetWorldRotation (stale _array_element) (Math|Rotator|Lerp(Rotator) (Utilities|Array|Get(acopy) (Variables|Default|GetSourceRotations) _array_index) "0, 0, 0" _returnvalue_3) false false))
      (if (not (<= (Utilities|Time|GetGameTimeinSeconds) (+ (Variables|Default|GetPositioningStartTime) (Variables|Default|GetPositioningDuration))))
        (CallFunction|LaunchPlates)))))

(fn ConstructionScript)