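; Boss pushback hazard that repels the player with an expanding flood splash.
; Player overlap starts the splash, disabling the trigger sphere while Tick lerps the flood collider and local height fog wider and lower over the splash duration, then resets them.
; Overlaps during the splash cancel aiming and launch the player away from the center.
; A second sphere runs a looping timer that damages and pushes the player while inside.
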(event OnComponentBeginOverlap(Sphere1)
  (params (OverlappedComponent :type Primitive%20Component%20Object%20Reference) (OtherActor :type Actor%20Object%20Reference) (OtherComp :type Primitive%20Component%20Object%20Reference) (OtherBodyIndex :type Integer) (bFromSweep :type Boolean) (SweepResult :type Hit%20Result%20Structure%20%28by%20ref%29))
  (if (== OtherActor (Variables|Default|GetPlayer))
    (bind _returnvalue (Utilities|Time|SetTimerbyEvent (delegate Custom|push) 0.3 true))))

(event OnComponentEndOverlap(Sphere1)
  (params (OverlappedComponent :type Primitive%20Component%20Object%20Reference) (OtherActor :type Actor%20Object%20Reference) (OtherComp :type Primitive%20Component%20Object%20Reference) (OtherBodyIndex :type Integer))
  (if (== OtherActor (Variables|Default|GetPlayer))
    (Utilities|Time|ClearandInvalidateTimerbyHandle (stale OnComponentBeginOverlap(Sphere1) _returnvalue))))

(event Custom|StartSplash
  (Rendering|SetVisibility (Variables|Default|GetFloodCollider) true false)
  (Variables|Default|SetSplashing true)
  (Variables|Default|SetSplashStart (Utilities|Time|GetGameTimeinSeconds))
  (Collision|SetCollisionEnabled (Variables|Default|GetSphere) "NoCollision")
  (Rendering|SetVisibility (Variables|Default|GetLocalHeightFog) true false))

(event Custom|EndSplash
  (Rendering|SetVisibility (Variables|Default|GetFloodCollider) false false)
  (Variables|Default|SetSplashing false)
  (Collision|SetCollisionEnabled (Variables|Default|GetSphere) "QueryOnly")
  (Transformation|SetWorldScale3D (Variables|Default|GetFloodCollider) (Math|Vector|MakeVector 0.3 0.3 3.0))
  (Rendering|SetVisibility (Variables|Default|GetLocalHeightFog) true false)
  (Transformation|SetWorldScale3D (Variables|Default|GetLocalHeightFog) (Math|Vector|MakeVector 275.0 275.0 5e+02))
  (Transformation|SetRelativeLocation (Variables|Default|GetLocalHeightFog) (Variables|Default|GetFogPosition) false false))

(event Custom|push
  (bind _player (Variables|Default|GetPlayer))
  (Default|DamagePlayer _player 1e+01)
  (Character|LaunchCharacter _player (* (Math|Vector|Normalize (- (Transformation|GetActorLocation _player) (Transformation|GetActorLocation))) (Variables|Default|GetPushForce)) false false))

(event EventBeginPlay
  (bind _asbp_third_person_character (Utilities|Casting|CastToBP_ThirdPersonCharacter (Game|GetPlayerCharacter 0))
    (:then
      (Variables|Default|SetPlayer _asbp_third_person_character)
      (Variables|Default|SetFogPosition (Variables|/Script/Engine.SceneComponent|GetRelativeLocation (Variables|Default|GetLocalHeightFog))))
    (:CastFailed
      (Development|PrintText "Could not cast player variable"))))

(event Collision|EventActorBeginOverlap
  (params (OtherActor :type Actor%20Object%20Reference))
  (bind _player (Variables|Default|GetPlayer))
  (if (== OtherActor (Variables|Default|GetPlayer))
    (if (Variables|Default|GetSplashing)
      (Default|EndAiming _player)
      (Character|LaunchCharacter _player (* (Math|Vector|Normalize (- (Transformation|GetActorLocation _player) (Transformation|GetActorLocation))) (Variables|Default|GetPushForce)) false false)
      (else
        (CallFunction|StartSplash)))))

(event EventTick
  (params (DeltaSeconds :type Float%20%28single-precision%29))
  (bind _returnvalue (Utilities|Time|GetGameTimeinSeconds))
  (bind _splashduration (Variables|Default|GetSplashDuration))
  (bind _fogposition (Variables|Default|GetFogPosition))
  (bind _splashstart (Variables|Default|GetSplashStart))
  (bind _returnvalue_2 (- _returnvalue _splashstart))
  (bind _returnvalue_3 (/ _returnvalue_2 _splashduration))
  (bind _returnvalue_4 (Math|Float|Lerp 0.3 1.3 _returnvalue_3))
  (bind _returnvalue_5 (Math|Float|Lerp 275.0 1.2e+03 _returnvalue_3))
  (if (Variables|Default|GetSplashing)
    (Transformation|SetWorldScale3D (Variables|Default|GetFloodCollider) (Math|Vector|MakeVector _returnvalue_4 _returnvalue_4 (Math|Float|Lerp 3.0 0.0 _returnvalue_3)))
    (Transformation|SetWorldScale3D (Variables|Default|GetLocalHeightFog) (Math|Vector|MakeVector _returnvalue_5 _returnvalue_5 5e+02))
    (Transformation|SetRelativeLocation (Variables|Default|GetLocalHeightFog) (Math|Vector|MakeVector (.x _fogposition) (.y _fogposition) (Math|Float|Lerp 575.0 0.0 _returnvalue_3)) false false)
    (if (>= (Utilities|Time|GetGameTimeinSeconds) (+ (Variables|Default|GetSplashStart) (Variables|Default|GetSplashDuration)))
      (CallFunction|EndSplash))))

(fn ConstructionScript)