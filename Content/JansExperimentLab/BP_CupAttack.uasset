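; Teacup attack actor that sends three spinning cups along spline paths and damages the player on overlap.
; On BeginPlay it randomly yaws each spline within its own sector, then staggers three randomly timed launches.
; Timelines move each cup along its spline at a lap-duration-based rate, repeating up to MaxLaps before destroying cup and spline.
; Tick spins the cups and keeps the actor's height locked just above the BP_LargePlate.
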(event Custom|LaunchCup1
  (CallFunction|Timeline1)
  (Components|Timeline|SetPlayRate (Variables|Default|GetMove1) (/ 1.0 (Variables|Default|GetTeacupLapDuration))))

(event Custom|LaunchCup2
  (CallFunction|Timeline2)
  (Components|Timeline|SetPlayRate (Variables|Default|GetMove2) (/ 1.0 (Variables|Default|GetTeacupLapDuration))))

(event Custom|LaunchCup3
  (CallFunction|Timeline3)
  (Components|Timeline|SetPlayRate (Variables|Default|GetMove3) (/ 1.0 (Variables|Default|GetTeacupLapDuration))))

(event Custom|Timeline1
  (bind _laps1 (Variables|Default|GetLaps1))
  (bind _alpha (Timeline|Move1 PlayFromStart)
    (:Update
      (Transformation|SetWorldLocation (Variables|Default|GetSM_Teacup1) (Spline|GetLocationatTime (Variables|Default|GetSpline1) _alpha "World" false) false false))
    (:Finished
      (Math|Integer|IncrementInt _laps1
        (:%20%20
          (if (<= _laps1 (Variables|Default|GetMaxLaps))
            (Timeline|Move1 PlayFromStart)
            (else
              (Components|DestroyComponent (Variables|Default|GetSM_Teacup1))
              (Components|DestroyComponent (Variables|Default|GetSpline1)))))))))

(event Custom|Timeline2
  (bind _laps2 (Variables|Default|GetLaps2))
  (bind _alpha (Timeline|Move2 PlayFromStart)
    (:Update
      (Transformation|SetWorldLocation (Variables|Default|GetSM_Teacup2) (Spline|GetLocationatTime (Variables|Default|GetSpline2) _alpha "World" false) false false))
    (:Finished
      (Math|Integer|IncrementInt _laps2
        (:%20%20
          (if (<= _laps2 (Variables|Default|GetMaxLaps))
            (Timeline|Move2 PlayFromStart)
            (else
              (Components|DestroyComponent (Variables|Default|GetSM_Teacup2))
              (Components|DestroyComponent (Variables|Default|GetSpline2)))))))))

(event Custom|Timeline3
  (bind _laps3 (Variables|Default|GetLaps3))
  (bind _alpha (Timeline|Move3 PlayFromStart)
    (:Update
      (Transformation|SetWorldLocation (Variables|Default|GetSM_Teacup3) (Spline|GetLocationatTime (Variables|Default|GetSpline3) _alpha "World" false) false false))
    (:Finished
      (Math|Integer|IncrementInt _laps3
        (:%20%20
          (if (<= _laps3 (Variables|Default|GetMaxLaps))
            (Timeline|Move3 PlayFromStart)
            (else
              (Components|DestroyComponent (Variables|Default|GetSM_Teacup3))
              (Components|DestroyComponent (Variables|Default|GetSpline3)))))))))

(event EventBeginPlay
  (bind _returnvalue (Actor|GetActorOfClass "/Game/JansExperimentLab/BP_LargePlate.BP_LargePlate_C"))
  (if (Utilities|IsValid _returnvalue)
    (Variables|Default|SetPlateActor _returnvalue))
  (bind _asbp_third_person_character (Utilities|Casting|CastToBP_ThirdPersonCharacter (Game|GetPlayerCharacter 0))
    (:then
      (Variables|Default|SetPlayer _asbp_third_person_character)
      (Transformation|SetWorldRotation (Variables|Default|GetSpline1) (Math|Rotator|MakeRotator 0.0 0.0 (Math|Random|RandomFloatinRange 2e+01 1e+02)) false false)
      (Transformation|SetWorldRotation (Variables|Default|GetSpline2) (Math|Rotator|MakeRotator 0.0 0.0 (Math|Random|RandomFloatinRange 1.4e+02 2.2e+02)) false false)
      (Transformation|SetWorldRotation (Variables|Default|GetSpline3) (Math|Rotator|MakeRotator 0.0 0.0 (Math|Random|RandomFloatinRange 2.6e+02 3.4e+02)) false false)
      (Utilities|Time|SetTimerbyEvent (delegate Custom|LaunchCup1) (Math|Random|RandomFloatinRange 0.0 1.5))
      (Utilities|Time|SetTimerbyEvent (delegate Custom|LaunchCup2) (Math|Random|RandomFloatinRange 2.0 3.5))
      (Utilities|Time|SetTimerbyEvent (delegate Custom|LaunchCup3) (Math|Random|RandomFloatinRange 4.0 5.5)))
    (:CastFailed
      (Development|PrintText "Couldn't cast character"))))

(event Collision|EventActorBeginOverlap
  (params (OtherActor :type Actor%20Object%20Reference))
  (bind _player (Variables|Default|GetPlayer))
  (if (== OtherActor _player)
    (Default|DamagePlayer _player (Variables|Default|GetCupDamage))))

(event EventTick
  (params (DeltaSeconds :type Float%20%28single-precision%29))
  (bind _returnvalue (Transformation|GetActorLocation))
  (bind _plateactor (Variables|Default|GetPlateActor))
  (bind _cuprotationspeed (Variables|Default|GetCupRotationSpeed))
  (bind _sm_teacup1 (Variables|Default|GetSM_Teacup1))
  (bind _sm_teacup2 (Variables|Default|GetSM_Teacup2))
  (bind _sm_teacup3 (Variables|Default|GetSM_Teacup3))
  (bind _returnvalue_2 (* DeltaSeconds _cuprotationspeed))
  (Utilities|FlowControl|Sequence
    (:then_0
      (if (Utilities|IsValid _sm_teacup1)
        (Transformation|AddLocalRotation _sm_teacup1 (Math|Rotator|MakeRotator 0.0 0.0 _returnvalue_2) false false)))
    (:then_1
      (if (Utilities|IsValid _sm_teacup2)
        (Transformation|AddLocalRotation _sm_teacup2 (Math|Rotator|MakeRotator 0.0 0.0 _returnvalue_2) false false)))
    (:then_2
      (if (Utilities|IsValid _sm_teacup3)
        (Transformation|AddLocalRotation _sm_teacup3 (Math|Rotator|MakeRotator 0.0 0.0 _returnvalue_2) false false)))
    (:then_3
      (if (Utilities|IsValid _plateactor)
        (Transformation|SetActorLocation (Math|Vector|MakeVector (.x _returnvalue) (.y _returnvalue) (+ (.z (Transformation|GetActorLocation _plateactor)) 18.4)) false false)))))

(fn ConstructionScript)