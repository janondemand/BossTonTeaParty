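; BP_SaucerSpawner spawns three BP_Saucer actors when play begins and collects them in PlateGroup.
; Each saucer receives a launch position and an X-offset start position derived from its own marker components, plus a shared rotation pivot.
; The spawner also passes rotation speed, positioning duration and launch speed, leaving movement to the saucers.
; It records its start time and has no active Tick logic.
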(event EventBeginPlay
  (bind _returnvalue (Transformation|GetActorLocation))
  (bind _returnvalue_2 (Transformation|GetActorLocation))
  (bind _returnvalue_3 (Transformation|GetActorLocation))
  (bind _platestart0 (Variables|Default|GetPlateStart0))
  (bind _platestart1 (Variables|Default|GetPlateStart1))
  (bind _platestart2 (Variables|Default|GetPlateStart2))
  (bind _relativelocation (Variables|/Script/Engine.SceneComponent|GetRelativeLocation _platestart0))
  (bind _relativelocation_2 (Variables|/Script/Engine.SceneComponent|GetRelativeLocation _platestart1))
  (bind _relativelocation_3 (Variables|/Script/Engine.SceneComponent|GetRelativeLocation _platestart2))
  (Variables|Default|SetStartTime (Utilities|Time|GetGameTimeinSeconds))
  (bind _returnvalue_4 (Game|SpawnActorfromClass "/Game/JansExperimentLab/BP_Saucer.BP_Saucer_C" (Transformation|GetActorTransform) "Undefined" "MultiplyWithRoot" 0 (+ _returnvalue_2 (Variables|/Script/Engine.SceneComponent|GetRelativeLocation (Variables|Default|GetLaunchPosition0))) (Transformation|GetWorldLocation (Variables|Default|GetSaucerRotationPivot)) (Variables|Default|GetRotationSpeed) (Variables|Default|GetPositioningDuration) (Variables|Default|GetLaunchSpeed) (+ (Math|Vector|MakeVector -6e+02 (.y _relativelocation) (.z _relativelocation)) _returnvalue_2) 0))
  (Utilities|Array|Add (Variables|Default|GetPlateGroup) _returnvalue_4)
  (bind _returnvalue_5 (Game|SpawnActorfromClass "/Game/JansExperimentLab/BP_Saucer.BP_Saucer_C" (Transformation|GetActorTransform) "Undefined" "MultiplyWithRoot" 0 (+ _returnvalue_3 (Variables|/Script/Engine.SceneComponent|GetRelativeLocation (Variables|Default|GetLaunchPosition1))) (+ (Transformation|GetActorLocation) (Variables|/Script/Engine.SceneComponent|GetRelativeLocation (Variables|Default|GetSaucerRotationPivot))) (Variables|Default|GetRotationSpeed) (Variables|Default|GetPositioningDuration) (Variables|Default|GetLaunchSpeed) (+ (Math|Vector|MakeVector -6e+02 (.y _relativelocation_2) (.z _relativelocation_2)) _returnvalue_3) 0))
  (Utilities|Array|Add (Variables|Default|GetPlateGroup) _returnvalue_5)
  (bind _returnvalue_6 (Game|SpawnActorfromClass "/Game/JansExperimentLab/BP_Saucer.BP_Saucer_C" (Transformation|GetActorTransform) "Undefined" "MultiplyWithRoot" 0 (+ _returnvalue (Variables|/Script/Engine.SceneComponent|GetRelativeLocation (Variables|Default|GetLaunchPosition2))) (Transformation|GetWorldLocation (Variables|Default|GetSaucerRotationPivot)) (Variables|Default|GetRotationSpeed) (Variables|Default|GetPositioningDuration) (Variables|Default|GetLaunchSpeed) (+ (Math|Vector|MakeVector -6e+02 (.y _relativelocation_3) (.z _relativelocation_3)) _returnvalue) 0))
  (Utilities|Array|Add (Variables|Default|GetPlateGroup) _returnvalue_6))

(event Collision|EventActorBeginOverlap
  (params (OtherActor :type Actor%20Object%20Reference)))

(event EventTick
  (params (DeltaSeconds :type Float%20%28single-precision%29)))

(fn ConstructionScript)