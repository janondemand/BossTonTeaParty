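; Prototype enemy saucer that attacks the player, dealing damage and destroying itself on overlap.
; Tick runs a time-driven state machine: it waits while Shielding, pitches the mesh upright while Positioning, then Launching pauses before lerping from the launch point toward the player's live location.
; Incoming damage reduces health, swapping to a cracked mesh until health runs out and the saucer is destroyed.
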(event EventBeginPlay
  (bind _asbp_third_person_character (Utilities|Casting|CastToBP_ThirdPersonCharacter (Game|GetPlayerCharacter 0)))
  (Variables|Default|SetPlayer _asbp_third_person_character)
  (Variables|Default|SetStartTime (Utilities|Time|GetGameTimeinSeconds))
  (Variables|Default|SetCurrentSaucerMesh (Variables|Default|GetSM_Saucer_CorrectScale)))

(event Collision|EventActorBeginOverlap
  (params (OtherActor :type Actor%20Object%20Reference))
  (bind _player (Variables|Default|GetPlayer))
  (if (== OtherActor _player)
    (Default|DamagePlayer _player 1e+01)
    (Actor|DestroyActor)))

(event EventTick
  (params (DeltaSeconds :type Float%20%28single-precision%29))
  (bind _returnvalue (Utilities|Time|GetGameTimeinSeconds))
  (bind _launchdelay (Variables|Default|GetLaunchDelay))
  (switch Utilities|FlowControl|Switch|SwitchonEnum_PlateState (Variables|Default|GetSaucerState)
    (:NewEnumerator0
      (if (>= _returnvalue (+ (Variables|Default|GetStartTime) (Variables|Default|GetDelayUntilAttack)))
        (bind _output_get (Variables|Default|SetPositioningStart _returnvalue))
        (Variables|Default|SetPositioningEnd (+ (Variables|Default|GetPositioningTime) _output_get))
        (Variables|Default|SetSaucerState "NewEnumerator1")))
    (:NewEnumerator1
      (if (< (Utilities|Time|GetGameTimeinSeconds) (+ (Variables|Default|GetPositioningStart) (Variables|Default|GetPositioningTime)))
        (Transformation|SetRelativeRotation (Variables|Default|GetCurrentSaucerMesh) (Math|Rotator|MakeRotator 0.0 (Math|Float|Lerp 0.0 9e+01 (/ (- (Utilities|Time|GetGameTimeinSeconds) (Variables|Default|GetPositioningStart)) (Variables|Default|GetPositioningTime))) 0.0) false false)
        (else
          (Variables|Default|SetLaunchLocation (Transformation|GetActorLocation))
          (Variables|Default|SetTimeLaunched (Utilities|Time|GetGameTimeinSeconds))
          (Variables|Default|SetSaucerState "NewEnumerator2"))))
    (:NewEnumerator2
      (if (>= (- (Utilities|Time|GetGameTimeinSeconds) (Variables|Default|GetTimeLaunched)) _launchdelay)
        (Transformation|SetActorLocation (Math|Vector|Lerp(Vector) (Variables|Default|GetLaunchLocation) (Transformation|GetActorLocation (Variables|Default|GetPlayer)) (/ (- (Utilities|Time|GetGameTimeinSeconds) (+ (Variables|Default|GetTimeLaunched) _launchdelay)) (Variables|Default|GetLaunchDuration))) false false)))))

(event EventDamage
  (params (DamageAmount :type Float%20%28double-precision%29))
  (switch Utilities|FlowControl|Switch|SwitchonEnum_PlateState "NewEnumerator0"
    (:NewEnumerator0
      (bind _output_get (Variables|Default|SetSaucerHealth (- (Variables|Default|GetSaucerHealth) DamageAmount)))
      (if (<= _output_get 0.0)
        (Actor|DestroyActor)
        (else
          (Rendering|SetVisibility (Variables|Default|GetSM_CrackedSaucer) true false)
          (Rendering|SetVisibility (Variables|Default|GetSM_Saucer_CorrectScale) false false)
          (Variables|Default|SetCurrentSaucerMesh (Variables|Default|GetSM_CrackedSaucer)))))))

(fn ConstructionScript)