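; BP_TeaFlood is a flood hazard actor that rises, stays, recedes and damages the player while they overlap it.
; Tick runs a Warning, Flooding, Staying and Receding state machine timed from game time, with a warning field shown from BeginPlay until flooding starts.
; Lerps move the actor and local height fog up and back down, destroying the actor once its Z reaches zero.
; A looping timer applies damage during overlap.
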(event Custom|Flood
  (Variables|Default|SetFloodState "NewEnumerator0")
  (Variables|Default|SetStartTime (Utilities|Time|GetGameTimeinSeconds))
  (Rendering|SetVisibility (Variables|Default|GetWarningField) false false))

(event Custom|Staying
  (Variables|Default|SetFloodState "NewEnumerator1")
  (Variables|Default|SetStartTime (Utilities|Time|GetGameTimeinSeconds)))

(event Custom|Receding
  (Variables|Default|SetFloodState "NewEnumerator2")
  (Variables|Default|SetStartTime (Utilities|Time|GetGameTimeinSeconds)))

(event Custom|damage
  (Default|DamagePlayer (Variables|Default|GetPlayer) 1e+01))

(event EventBeginPlay
  (bind _asbp_third_person_character (Utilities|Casting|CastToBP_ThirdPersonCharacter (Game|GetPlayerCharacter 0)))
  (Variables|Default|SetPlayer _asbp_third_person_character)
  (Variables|Default|SetStartTime (Utilities|Time|GetGameTimeinSeconds))
  (Variables|Default|SetStartLocation (Transformation|GetActorLocation))
  (Rendering|SetVisibility (Variables|Default|GetWarningField) true false))

(event Collision|EventActorBeginOverlap
  (params (OtherActor :type Actor%20Object%20Reference))
  (if (== OtherActor (Variables|Default|GetPlayer))
    (bind _returnvalue (Utilities|Time|SetTimerbyEvent (delegate Custom|damage) 0.1 true))))

(event EventTick
  (params (DeltaSeconds :type Float%20%28single-precision%29))
  (bind _startlocation (Variables|Default|GetStartLocation))
  (bind _localheightfog (Variables|Default|GetLocalHeightFog))
  (bind _localheightfog_2 (Variables|Default|GetLocalHeightFog))
  (bind _startlocation_2 (Variables|Default|GetStartLocation))
  (bind _returnvalue (Transformation|GetWorldLocation _localheightfog))
  (bind _returnvalue_2 (Transformation|GetWorldLocation _localheightfog_2))
  (switch Utilities|FlowControl|Switch|SwitchonEnum_FloodState (Variables|Default|GetFloodState)
    (:NewEnumerator0
      (if (< (- (Utilities|Time|GetGameTimeinSeconds) (Variables|Default|GetStartTime)) (Variables|Default|GetFloodingDuration))
        (Transformation|SetActorLocation (Math|Vector|MakeVector (.x _startlocation) (.y _startlocation) (Math|Float|Lerp (.z (Variables|Default|GetStartLocation)) (Variables|Default|GetFloodHeight) (/ (- (Utilities|Time|GetGameTimeinSeconds) (Variables|Default|GetStartTime)) (Variables|Default|GetFloodingDuration)))) false false)
        (Transformation|SetWorldLocation _localheightfog_2 (Math|Vector|MakeVector (.x _returnvalue_2) (.y _returnvalue_2) (Math|Float|Lerp -5e+02 (Variables|Default|GetFloodHeight) (/ (- (Utilities|Time|GetGameTimeinSeconds) (Variables|Default|GetStartTime)) (Variables|Default|GetFloodingDuration)))) false false)
        (else
          (CallFunction|Staying))))
    (:NewEnumerator1
      (if (not (< (- (Utilities|Time|GetGameTimeinSeconds) (Variables|Default|GetStartTime)) (Variables|Default|GetStayDuration)))
        (CallFunction|Receding)))
    (:NewEnumerator2
      (Transformation|SetActorLocation (Math|Vector|MakeVector (.x _startlocation_2) (.y _startlocation_2) (Math|Float|Lerp (Variables|Default|GetFloodHeight) (.z (Variables|Default|GetStartLocation)) (/ (- (Utilities|Time|GetGameTimeinSeconds) (Variables|Default|GetStartTime)) (Variables|Default|GetFloodingDuration)))) false false)
      (Transformation|SetWorldLocation _localheightfog (Math|Vector|MakeVector (.x _returnvalue) (.y _returnvalue) (Math|Float|Lerp (Variables|Default|GetFloodHeight) -5e+02 (/ (- (Utilities|Time|GetGameTimeinSeconds) (Variables|Default|GetStartTime)) (Variables|Default|GetFloodingDuration)))) false false)
      (if (<= (.z (Transformation|GetActorLocation)) 0.0)
        (Actor|DestroyActor)))
    (:NewEnumerator3
      (if (not (< (- (Utilities|Time|GetGameTimeinSeconds) (Variables|Default|GetStartTime)) (Variables|Default|GetFloodingDuration)))
        (CallFunction|Flood)))))

(event Collision|EventActorEndOverlap
  (params (OtherActor :type Actor%20Object%20Reference))
  (if (== OtherActor (Variables|Default|GetPlayer))
    (Utilities|Time|ClearandInvalidateTimerbyHandle (stale Collision|EventActorBeginOverlap _returnvalue))))

(fn ConstructionScript)