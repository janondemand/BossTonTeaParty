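; BP_Temporary is an experimental Blueprint holding a DrawProjectilePath function that previews a slingshot's launch arc; its own event graph is empty.
; Each call raises SlingshotPower by a frame-time-scaled step without exceeding the maximum, then predicts a projectile path along Arrow1's forward vector.
; It destroys the previous arc's components and spawns a static mesh component at every predicted point, tracking them in LastArc.
; Segment rotation logic is left unused.
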(event EventBeginPlay)

(event Collision|EventActorBeginOverlap
  (params (OtherActor :type Actor%20Object%20Reference)))

(event EventTick
  (params (DeltaSeconds :type Float%20%28single-precision%29)))

(fn ConstructionScript)

(fn DrawProjectilePath
  (bind _slingshotmaxpower (Variables|Default|GetSlingshotMaxPower))
  (bind _lastarc (Variables|Default|GetLastArc))
  (if (<= (+ (Variables|Default|GetSlingshotPower) (* (Variables|Default|GetSlingshotMaxPullTime) (- _slingshotmaxpower (Variables|Default|GetSlingshotMinPower)) (Utilities|Time|GetWorldDeltaSeconds))) _slingshotmaxpower)
    (Variables|Default|SetSlingshotPower (+ (Variables|Default|GetSlingshotPower) (* (Variables|Default|GetSlingshotMaxPullTime) (- _slingshotmaxpower (Variables|Default|GetSlingshotMinPower)) (Utilities|Time|GetWorldDeltaSeconds)))))
  (bind _outpathpositions (Class|GameplayStatics|BlueprintPredictProjectilePathbyTraceChannel (Transformation|GetWorldLocation (Variables|Default|GetArrow1)) (* (Math|Vector|GetForwardVector (Variables|Default|GetArrow1)) (Variables|Default|GetSlingshotPower)) true 1e+01 "ECC_Visibility" false (Utilities|Array|MakeArray self) "None" 5.0 15.0 4.0))
  (for _array_element _lastarc
    (Components|DestroyComponent _array_element))
  (Utilities|Array|Clear _lastarc)
  (for (_array_element_2 _array_index) _outpathpositions
    (bind _returnvalue (AddComponent|AddStaticMeshComponent false))
    (Transformation|SetWorldLocation _returnvalue _array_element_2 false false)
    (Utilities|Array|Add (Variables|Default|GetLastArc) _returnvalue)))