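; BP_LargePlate is a plate actor that rises and falls with a tea flood.
; Overlapping an actor tagged "teaflood" stores that actor and sets Flooded.
; While flooded, Tick keeps the starting X and Y and sets Z to the starting Z plus the flood actor's world Z.
; End overlap requires the flood actor to be both valid and invalid, so Flooded never clears.
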(event EventBeginPlay
  (Variables|Default|SetStartLocation (Transformation|GetActorLocation)))

(event Collision|EventActorBeginOverlap
  (params (OtherActor :type Actor%20Object%20Reference))
  (if (Actor|ActorHasTag OtherActor "teaflood")
    (Variables|Default|SetFlooded true)
    (Variables|Default|SetTeafloodActor OtherActor)))

(event EventTick
  (params (DeltaSeconds :type Float%20%28single-precision%29))
  (bind _startlocation (Variables|Default|GetStartLocation))
  (if (Variables|Default|GetFlooded)
    (if (Utilities|IsValid (Variables|Default|GetTeafloodActor))
      (Transformation|SetActorLocation (Math|Vector|MakeVector (.x _startlocation) (.y _startlocation) (+ (.z _startlocation) (.z (Transformation|GetActorLocation (Variables|Default|GetTeafloodActor))))) false false))))

(event Collision|EventActorEndOverlap
  (params (OtherActor :type Actor%20Object%20Reference))
  (if (Utilities|IsValid (Variables|Default|GetTeafloodActor))
    (if (Actor|ActorHasTag OtherActor "teaflood")
      (if (not (Utilities|IsValid (Variables|Default|GetTeafloodActor)))
        (Variables|Default|SetFlooded false)))))

(fn ConstructionScript)