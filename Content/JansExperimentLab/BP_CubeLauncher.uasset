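; BP_CubeLauncher is an experimental actor whose cube homes in on the player character.
; BeginPlay caches the player, and Tick turns the cube to face them every frame.
; LaunchCube clears IsTargeting, after which Tick also moves the cube forward at CubeMoveSpeed without sweeping, so it keeps tracking in flight.
; A physics-impulse launch using SetSimulatePhysics and AddForce is left unconnected.
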(event Custom|LaunchCube
  (Variables|Default|SetIsTargeting false))

(event EventBeginPlay
  (bind _asbp_third_person_character (Utilities|Casting|CastToBP_ThirdPersonCharacter (Game|GetPlayerCharacter 0)))
  (Variables|Default|SetPlayerCharacter _asbp_third_person_character))

(event Collision|EventActorBeginOverlap
  (params (OtherActor :type Actor%20Object%20Reference)))

(event EventTick
  (params (DeltaSeconds :type Float%20%28single-precision%29))
  (bind _cube (Variables|Default|GetCube))
  (Transformation|SetWorldTransform (Variables|Default|GetCube) (Class|KismetAnimationLibrary|Lookat (Transformation|GetWorldTransform (Variables|Default|GetCube)) (Transformation|GetActorLocation (Variables|Default|GetPlayerCharacter)) "1.000000,0.000000,0.000000" false "0.000000,0.000000,0.000000" 0.0) false false)
  (if (not (Variables|Default|GetIsTargeting))
    (Transformation|AddWorldOffset _cube (* (Math|Vector|GetForwardVector _cube) (* (Variables|Default|GetCubeMoveSpeed) DeltaSeconds)) false false)))

(fn ConstructionScript)