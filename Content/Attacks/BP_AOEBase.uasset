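; BP_AOEBase is a base actor for area-of-effect attacks that activate after a delay.
; On BeginPlay it starts a timer of TimeToActivate and caches the third-person player character.
; When the timer fires, it teleport-free moves its Box by OffsetAfterActive and swaps the Cube material to show the active state.
; No overlap or damage logic is present here.
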(event Custom|EnableTrigger
  (bind _box (Variables|Default|GetBox))
  (Transformation|SetWorldLocation _box (+ (Transformation|GetWorldLocation _box) (Variables|Default|GetOffsetAfterActive)) false false)
  (Rendering|Material|SetMaterial (Variables|Default|GetCube) 0 (Variables|Default|GetMaterialAfterTrigger)))

(event EventBeginPlay
  (Utilities|Time|SetTimerbyEvent (delegate Custom|EnableTrigger) (Variables|Default|GetTimeToActivate))
  (bind _asbp_third_person_character (Utilities|Casting|CastToBP_ThirdPersonCharacter (Game|GetPlayerCharacter 0)))
  (bind _output_get (Variables|Default|SetAs%20BP%20Third%20Person%20Character _asbp_third_person_character))
  (Utilities|IsValid _output_get
    (:Is%20Not%20Valid
      (Development|PrintString "Cant find player"))))

(event Collision|EventActorBeginOverlap
  (params (OtherActor :type Actor%20Object%20Reference)))

(event EventTick
  (params (DeltaSeconds :type Float%20%28single-precision%29)))

(fn ConstructionScript)