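; BP_AOESlow is an area-of-effect attack actor that slows the player character while inside its Box volume.
; On begin overlap with player 0, it saves the third-person character's MaxWalkSpeed and sets it to that value minus SpeedPenalty.
; On end overlap, it restores the saved speed and resets the stored value to zero.
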(event OnComponentBeginOverlap(Box)
  (params (OverlappedComponent :type Primitive%20Component%20Object%20Reference) (OtherActor :type Actor%20Object%20Reference) (OtherComp :type Primitive%20Component%20Object%20Reference) (OtherBodyIndex :type Integer) (bFromSweep :type Boolean) (SweepResult :type Hit%20Result%20Structure%20%28by%20ref%29))
  (bind _as_bp_third_person_character (Variables|Default|GetAs%20BP%20Third%20Person%20Character))
  (bind _charactermovement (Variables|/Script/Engine.Character|GetCharacterMovement _as_bp_third_person_character))
  ;[1 1 1] Slows player down if they enter the area
  (if (== OtherActor (Game|GetPlayerCharacter 0))
    (bind _output_get (Variables|Default|SetSaved%20Max%20Walk%20Speed (Variables|/Script/Engine.CharacterMovementComponent|GetMaxWalkSpeed _charactermovement)))
    (Variables|/Script/Engine.CharacterMovementComponent|SetMaxWalkSpeed _charactermovement (- _output_get (Variables|Default|GetSpeedPenalty)))))

(event OnComponentEndOverlap(Box)
  (params (OverlappedComponent :type Primitive%20Component%20Object%20Reference) (OtherActor :type Actor%20Object%20Reference) (OtherComp :type Primitive%20Component%20Object%20Reference) (OtherBodyIndex :type Integer))
  ;[1 1 1] Reverts to normal speed when leaving
  (if (== OtherActor (Variables|Default|GetAs%20BP%20Third%20Person%20Character))
    (Variables|/Script/Engine.CharacterMovementComponent|SetMaxWalkSpeed (Variables|/Script/Engine.Character|GetCharacterMovement (Variables|Default|GetAs%20BP%20Third%20Person%20Character)) (Variables|Default|GetSaved%20Max%20Walk%20Speed))
    (Variables|Default|SetSaved%20Max%20Walk%20Speed 0.0)))

(event EventBeginPlay
  (|CallParentFunction) ; This node is disabled and will not be called.\nDrag off pins to build functionality.
)

(event Collision|EventActorBeginOverlap
  (params (OtherActor :type Actor%20Object%20Reference))
  (|CallParentFunction OtherActor) ; This node is disabled and will not be called.\nDrag off pins to build functionality.
)

(event EventTick
  (params (DeltaSeconds :type Float%20%28single-precision%29))
  (|CallParentFunction DeltaSeconds) ; This node is disabled and will not be called.\nDrag off pins to build functionality.
)

(fn ConstructionScript
  (|CallParentFunction))