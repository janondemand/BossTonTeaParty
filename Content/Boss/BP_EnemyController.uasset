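; AI controller that makes a BP_EnemyBase pawn patrol the points of a BP_SplinePath in the level.
; After a short delay on BeginPlay it caches the pawn and the first spline path found, then starts Patrol.
; Patrol runs AI MoveTo to the target spline point and, on success only, advances or wraps the index and calls itself again.
; An unconnected Timeline-based approach to moving along spline distance remains unused.
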(event Custom|Patrol
  (bind _splineref (Variables|Default|GetSplineRef))
  (Utilities|IsValid _splineref
    (:Is%20Valid
      (AI|AIMoveTo (Variables|Default|GetAs%20BP%20Enemy%20Base) (Spline|GetLocationatSplinePoint (Variables|/Game/Boss/BP_SplinePath.BP_SplinePath_C|GetSpline _splineref) (Variables|Default|GetTarget) "World") 0 5.0 false
        (:OnSuccess
          (if (== (Variables|Default|GetTarget) (Spline|GetNumberOfSplinePoints (Variables|/Game/Boss/BP_SplinePath.BP_SplinePath_C|GetSpline (Variables|Default|GetSplineRef))))
            (Variables|Default|SetTarget 0)
            (else
              (Math|Integer|IncrementInt (Variables|Default|GetTarget)
                (:%20%20
                  _))))
          (CallFunction|Patrol))))
    (:Is%20Not%20Valid
      (Development|PrintString "NO SPLINE REFRENCE FOUND!"))))

(event EventBeginPlay
  (Utilities|FlowControl|Delay 0.2)
  (bind _asbp_enemy_base (Utilities|Casting|CastToBP_EnemyBase (Pawn|GetControlledPawn)))
  (Variables|Default|SetAs%20BP%20Enemy%20Base _asbp_enemy_base)
  (Utilities|FlowControl|Sequence
    (:then_0
      (bind _outactors (Actor|GetAllActorsOfClass "/Game/Boss/BP_SplinePath.BP_SplinePath_C"))
      (bind _output_get (Variables|Default|SetSplineRef (Utilities|Array|Get(acopy) _outactors)))
      (Utilities|IsValid _output_get
        (:Is%20Not%20Valid
          (Development|PrintString "NO SPLINE REFRENCE FOUND!"))))
    (:then_1
      (CallFunction|Patrol))))

(event EventTick
  (params (DeltaSeconds :type Float%20%28single-precision%29)))

(fn ConstructionScript)