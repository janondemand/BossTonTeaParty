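; AI controller for the first phase of a boss fight, which starts and drives the boss behavior tree.
; On possession it waits briefly, runs BT_Phase1, stores the player character in the blackboard, then sets the Wait state and an initial phase.
; Helper functions write the boss state (Normal, Moving, Vulnerable, Wait) and phase enums to blackboard keys for the tree to read.
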(event EventBeginPlay)

(event EventTick
  (params (DeltaSeconds :type Float%20%28single-precision%29)))

(event EventPossess
  (params (PossessedPawn :type Pawn%20Object%20Reference))
  (Utilities|FlowControl|Delay 0.2)
  (AI|RunBehaviorTree "/Game/Boss/BT_Phase1.BT_Phase1")
  (AI|Components|Blackboard|SetValueasObject (Variables|Default|GetBlackboard) (Utilities|Name|MakeLiteralName "PlayerRef") (Game|GetPlayerCharacter 0))
  (CallFunction|SetStateWait)
  (CallFunction|SetPhase "NewEnumerator0"))

(fn ConstructionScript)

(fn SetStateNormal
  (AI|Components|Blackboard|SetValueasEnum (Variables|Default|GetBlackboard) (Utilities|Name|MakeLiteralName "State") (Utilities|Enum|LiteralenumE_BossStates "NewEnumerator0")))

(fn SetStateMoving
  (AI|Components|Blackboard|SetValueasEnum (Variables|Default|GetBlackboard) (Utilities|Name|MakeLiteralName "State") (Utilities|Enum|LiteralenumE_BossStates "NewEnumerator1")))

(fn SetStateVulnerable
  (AI|Components|Blackboard|SetValueasEnum (Variables|Default|GetBlackboard) (Utilities|Name|MakeLiteralName "State") (Utilities|Enum|LiteralenumE_BossStates "NewEnumerator2")))

(fn SetStateWait
  (AI|Components|Blackboard|SetValueasEnum (Variables|Default|GetBlackboard) (Utilities|Name|MakeLiteralName "State") (Utilities|Enum|LiteralenumE_BossStates "NewEnumerator3")))

(fn SetPhase
  (params (Phase :type E_BossPhase%20Enum :default "NewEnumerator0"))
  (AI|Components|Blackboard|SetValueasEnum (Variables|Default|GetBlackboard) (Utilities|Name|MakeLiteralName "Phase") (Utilities|Enum|LiteralenumE_BossPhase Phase)))