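; Teapot boss actor with two phases that executes the attacks, node teleports and vulnerability windows used by its AI controller.
; Per-phase attack lists spawn cubes, saucers or tea floods, wait out their durations, then request a move after enough attacks.
; Damage updates the health bar, triggers a timed cracked-mesh window with a hit trigger, and switches to fogged phase 2 at a health threshold.
; Death only prints a message.
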(event Custom|AttacksPhase2
  (bind _afterlastdelayp2 (Variables|Attacks|GetAfterLastDelayP2))
  ;[1 1 1] attacks phase 2
  (switch Utilities|FlowControl|Switch|SwitchonE_Attacks (Utilities|Array|Get(acopy) (Variables|Attacks|GetAttacksToPerformP2) (Variables|Attacks|GetAttacksAmount))
    (:NewEnumerator2
      (Development|PrintString "no attack")
      (Utilities|FlowControl|Delay 2.0))
    (:NewEnumerator0
      (CallFunction|AttackCubes)
      (Utilities|FlowControl|Delay (+ (Utilities|Array|Get(acopy) (Variables|Attacks|GetAttackCubesIntervals) 2) _afterlastdelayp2)))
    (:NewEnumerator1
      (CallFunction|AttackPlates)
      (Utilities|FlowControl|Delay (+ (Utilities|Array|Get(acopy) (Variables|Attacks|GetAttackPlatesIntervals) 2) _afterlastdelayp2)))
    (:NewEnumerator3
      (bind _delay (CallFunction|AttackFlood))
      (Utilities|FlowControl|Delay (+ _delay _afterlastdelayp2)))
    (:NewEnumerator4
      (CallFunction|AttackCubes)
      (bind _delay_2 (CallFunction|AttackFlood))
      (Utilities|FlowControl|Delay (Math|Float|Max(Float) (+ (Utilities|Array|Get(acopy) (Variables|Attacks|GetAttackCubesIntervals) 2) _afterlastdelayp2) (+ _delay_2 _afterlastdelayp2)))))
  (CallFunction|FinishAttackExecute2))

(event Custom|Move%20to%20new%20node
  (bind _output_get (Variables|Default|Setselected%20rand (.OutItem (Utilities|Array|Random (Variables|Default|GetMoveNodes)))))
  (if (== _output_get (Variables|Default|GetCurrentNode))
    (CallFunction|MovetoNewNode)
    (else
      (Transformation|SetActorLocation (Transformation|GetWorldLocation (Variables|/Game/Boss/BP_MoveNode.BP_MoveNode_C|GetDefaultSceneRoot _output_get)) false true)
      (Variables|Default|SetCurrentNode _output_get))))

(event Custom|MakeVulnerable
  (bind _arrow4 (Variables|Default|GetArrow4))
  ;[1 1 1] Vulnerable logick
  (CallFunction|SetMeshCracked)
  (Utilities|FlowControl|DoOnce false
    (:Completed
      (bind _returnvalue (Game|SpawnActorfromClass "/Game/Boss/BP_VulnTrigger.BP_VulnTrigger_C" (Transformation|GetWorldTransform _arrow4) "Undefined" "MultiplyWithRoot" 0 self 0))
      (Transformation|AttachComponentToComponent _returnvalue _arrow4 "None" "KeepWorld" "KeepWorld" "KeepWorld" true)
      (bind _returnvalue_2 (Utilities|Time|SetTimerbyEvent (delegate Custom|StopVuln) (Variables|Vulnerable|GetVulnerableTime)))
      (Variables|Vulnerable|SetVulnTimer _returnvalue_2))))

(event Custom|StopVuln
  (bind _arrow4 (Variables|Default|GetArrow4))
  ;[1 1 1] Vulnerable logick
  (Variables|Vulnerable|SetIsVulnerable false)
  (Default|SetStateNormal (Variables|Default|GetAs%20BP%20Boss%20Phase%201Controller))
  (CallFunction|SetMeshNormal)
  (Transformation|DetachFromActor (stale Custom|MakeVulnerable _returnvalue) "KeepWorld" "KeepWorld" "KeepWorld")
  (Actor|DestroyActor (stale Custom|MakeVulnerable _returnvalue))
  (Utilities|FlowControl|DoOnce false) ; enters at Reset
)

(event Custom|StartBattle
  (Default|SetStateNormal (Variables|Default|GetAs%20BP%20Boss%20Phase%201Controller)))

(event Custom|Attack
  (bind _afterlastdelayp1 (Variables|Attacks|GetAfterLastDelayP1))
  ;[1 1 1] Attack logick
  (switch Utilities|FlowControl|Switch|SwitchonE_Attacks (Utilities|Array|Get(acopy) (Variables|Attacks|GetAttacksToPerformP1) (Variables|Attacks|GetAttacksAmount))
    (:NewEnumerator2
      (Development|PrintString "no attack")
      (Utilities|FlowControl|Delay 2.0))
    (:NewEnumerator0
      (CallFunction|AttackCubes)
      (Utilities|FlowControl|Delay (+ (Utilities|Array|Get(acopy) (Variables|Attacks|GetAttackCubesIntervals) 2) _afterlastdelayp1)))
    (:NewEnumerator1
      (CallFunction|AttackPlates)
      (Utilities|FlowControl|Delay (+ (Utilities|Array|Get(acopy) (Variables|Attacks|GetAttackPlatesIntervals) 2) _afterlastdelayp1)))
    (:NewEnumerator3
      (bind _delay (CallFunction|AttackFlood))
      (Utilities|FlowControl|Delay (+ _delay _afterlastdelayp1)))
    (:NewEnumerator4
      (CallFunction|AttackCubes)
      (bind _delay_2 (CallFunction|AttackFlood))
      (Utilities|FlowControl|Delay (Math|Float|Max(Float) (+ (Utilities|Array|Get(acopy) (Variables|Attacks|GetAttackCubesIntervals) 2) _afterlastdelayp1) (+ _delay_2 _afterlastdelayp1)))))
  (CallFunction|FinishAttackExecute))

(event EventBeginPlay
  (bind _self self)
  (bind _movenodes (Variables|Default|GetMoveNodes))
  (bind _arrow5 (Variables|Default|GetArrow5))
  (bind _returnvalue (Transformation|GetWorldTransform _arrow5))
  (bind _output (Utilities|Array|Get(acopy) _movenodes))
  (Utilities|FlowControl|Sequence
    (:then_0
      (bind _asbp_boss_phase_1controller (Utilities|Casting|CastToBP_BossPhase1Controller (AI|GetAIController _self)))
      (Variables|Default|SetAs%20BP%20Boss%20Phase%201Controller _asbp_boss_phase_1controller)
      (bind _returnvalue_2 (UserInterface|CreateWidget "/Game/HUD/WBP_BossBAr.WBP_BossBAr_C"))
      (bind _output_get (Variables|Default|SetBossBarRef _returnvalue_2))
      (UserInterface|Viewport|AddtoViewport _output_get 0)
      (CallFunction|SetMeshNormal)
      (Rendering|SetVisibility (Variables|Default|GetLocalHeightFog1) false false))
    (:then_1
      (for (_array_element _array_index) (Variables|Default|GetMoveNodes)
        (Utilities|IsValid _array_element
          (:Is%20Not%20Valid
            (Development|PrintString (Utilities|String|Append (Utilities|String|Append (Utilities|String|MakeLiteralString "NO NODE REF FOUND IN INDEX ") (Utilities|String|ToString(Integer) _array_index)) (Utilities|String|MakeLiteralString " ON THE BOSS PLEASE FIX!")) true true "(R=1.000000,G=0.000000,B=0.000000,A=1.000000)" 6.0)))))
    (:then_2
      (Transformation|SetActorLocation _self (Transformation|GetWorldLocation (Variables|/Game/Boss/BP_MoveNode.BP_MoveNode_C|GetDefaultSceneRoot _output)) false false)
      (Variables|Default|SetCurrentNode _output))
    (:then_3
      (Utilities|IsValid (Variables|Default|GetFloodSpawnArena)
        (:Is%20Not%20Valid
          (Development|PrintString "NO FLOOD LOCATION" true true "(R=1.000000,G=0.000000,B=0.000000,A=1.000000)" 6.0))))
    (:then_4
      (bind _returnvalue_3 (Game|SpawnActorfromClass "/Game/JansExperimentLab/BP_BossPushback.BP_BossPushback_C" (Math|Transform|MakeTransform (.location _returnvalue) (.rotation _returnvalue) "1.000000,1.000000,1.000000") "AlwaysSpawn" "MultiplyWithRoot" 0 0))
      (Transformation|AttachComponentToComponent _returnvalue_3 _arrow5 "None" "KeepWorld" "KeepWorld" "KeepWorld" true))))

(event Collision|EventActorBeginOverlap
  (params (OtherActor :type Actor%20Object%20Reference)))

(event EventTick
  (params (DeltaSeconds :type Float%20%28single-precision%29)))

(event EventDamage
  (params (DamageAmount :type Float%20%28double-precision%29))
  (bind _bossbarref (Variables|Default|GetBossBarRef))
  (bind _as_bp_boss_phase_1controller (Variables|Default|GetAs%20BP%20Boss%20Phase%201Controller))
  (bind _output_get (Variables|Default|SetCurrentHealth (- (Variables|Default|GetCurrentHealth) DamageAmount)))
  (if (<= _output_get 0.0)
    (Development|PrintString "Dead")
    (Default|UpdateBar _bossbarref (/ (Variables|Default|GetCurrentHealth) (Variables|Default|GetMaxHealth)))
    (else
      (Default|UpdateBar _bossbarref (/ (Variables|Default|GetCurrentHealth) (Variables|Default|GetMaxHealth)))
      (Utilities|FlowControl|Sequence
        (:then_0
          ;[1 1 1] Swich state once enought damage is dealt
          (Utilities|FlowControl|DoOnce false :!label _label
            (:Completed
              (if (<= (Variables|Default|GetCurrentHealth) (Variables|Default|GetHealthToPhase2))
                (Default|SetPhase _as_bp_boss_phase_1controller "NewEnumerator1")
                (Default|SetStateNormal _as_bp_boss_phase_1controller)
                ;;[1 1 1] avoid switching issues
                (Variables|Attacks|SetAttacksAmount 0)
                (Variables|Vulnerable|SetIsVulnerable false)
                (Variables|Vulnerable|SetDamageTaken 0.0)
                (Utilities|Time|ClearandInvalidateTimerbyHandle (Variables|Vulnerable|GetVulnTimer))
                (CallFunction|StopVuln)
                (Rendering|SetVisibility (Variables|Default|GetLocalHeightFog1) true false)
                (CallFunction|SetMeshNormal)
                (else
                  (goto _label Reset))))))
        (:then_1
          ;[1 1 1] Vulneable behavior
          (if (not (Variables|Vulnerable|GetIsVulnerable))
            (bind _output_get_2 (Variables|Vulnerable|SetDamageTaken (+ (Variables|Vulnerable|GetDamageTaken) DamageAmount)))
            (if (>= _output_get_2 (Variables|Vulnerable|GetDamageToVuln))
              (Variables|Vulnerable|SetDamageTaken 0.0)
              (Default|SetStateVulnerable (Variables|Default|GetAs%20BP%20Boss%20Phase%201Controller))
              (Variables|Vulnerable|SetIsVulnerable true))))
        (:then_2
          (Utilities|FlowControl|DoOnce false
            (:Completed
              (Default|SetStateNormal (Variables|Default|GetAs%20BP%20Boss%20Phase%201Controller)))))))))

(fn ConstructionScript)

(fn FinishAttackExecute
  (Default|CallAttackDoneP1)
  ;[1 1 1] every x attacks will switch state
  (bind _result (Math|Integer|IncrementInt (Variables|Attacks|GetAttacksAmount))
    (:%20%20
      (if (>= _result (Variables|Attacks|GetAttacksToSwichP1))
        (Variables|Attacks|SetAttacksAmount 0)
        (Default|SetStateMoving (Variables|Default|GetAs%20BP%20Boss%20Phase%201Controller))))))

(fn AttackPlates
  (bind _attackplatesintervals (Variables|Attacks|GetAttackPlatesIntervals))
  (bind _arrow1 (Variables|Default|GetArrow1))
  (bind _arrow2 (Variables|Default|GetArrow2))
  (bind _arrow3 (Variables|Default|GetArrow3))
  (bind _returnvalue (Transformation|GetWorldTransform _arrow1))
  (bind _returnvalue_2 (Transformation|GetWorldTransform _arrow2))
  (bind _returnvalue_3 (Transformation|GetWorldTransform _arrow3))
  (Game|SpawnActorfromClass "/Game/JansExperimentLab/BP_SaucerPrototype.BP_SaucerPrototype_C" (Math|Transform|MakeTransform (.location _returnvalue) (.rotation _returnvalue) "1.000000,1.000000,1.000000") "AlwaysSpawn" "MultiplyWithRoot" 0 (Utilities|Array|Get(acopy) _attackplatesintervals) 0)
  (Game|SpawnActorfromClass "/Game/JansExperimentLab/BP_SaucerPrototype.BP_SaucerPrototype_C" (Math|Transform|MakeTransform (.location _returnvalue_2) (.rotation _returnvalue_2) "1.000000,1.000000,1.000000") "AlwaysSpawn" "MultiplyWithRoot" 0 (Utilities|Array|Get(acopy) _attackplatesintervals 1) 0)
  (Game|SpawnActorfromClass "/Game/JansExperimentLab/BP_SaucerPrototype.BP_SaucerPrototype_C" (Math|Transform|MakeTransform (.location _returnvalue_3) (.rotation _returnvalue_3) "1.000000,1.000000,1.000000") "AlwaysSpawn" "MultiplyWithRoot" 0 (Utilities|Array|Get(acopy) _attackplatesintervals 2) 0))

(fn AttackCubes
  (bind _arrow3 (Variables|Default|GetArrow3))
  (bind _arrow1 (Variables|Default|GetArrow1))
  (bind _arrow2 (Variables|Default|GetArrow2))
  (bind _returnvalue (Transformation|GetWorldTransform _arrow1))
  (bind _returnvalue_2 (Transformation|GetWorldTransform _arrow2))
  (bind _returnvalue_3 (Transformation|GetWorldTransform _arrow3))
  (Game|SpawnActorfromClass "/Game/PatryksFolder/BossAttacks/Cubes/BP_Projectile_Base.BP_Projectile_Base_C" (Math|Transform|MakeTransform (.location _returnvalue) (.rotation _returnvalue) "1.000000,1.000000,1.000000") "AlwaysSpawn" "MultiplyWithRoot" 0 0.0 0.0 0 (Utilities|Array|Get(acopy) (Variables|Attacks|GetAttackCubesIntervals)) 0)
  (Game|SpawnActorfromClass "/Game/PatryksFolder/BossAttacks/Cubes/BP_Projectile_Base.BP_Projectile_Base_C" (Math|Transform|MakeTransform (.location _returnvalue_2) (.rotation _returnvalue_2) "1.000000,1.000000,1.000000") "AlwaysSpawn" "MultiplyWithRoot" 0 0.0 0.0 0 (Utilities|Array|Get(acopy) (Variables|Attacks|GetAttackCubesIntervals) 1) 0)
  (Game|SpawnActorfromClass "/Game/PatryksFolder/BossAttacks/Cubes/BP_Projectile_Base.BP_Projectile_Base_C" (Math|Transform|MakeTransform (.location _returnvalue_3) (.rotation _returnvalue_3) "1.000000,1.000000,1.000000") "AlwaysSpawn" "MultiplyWithRoot" 0 0.0 0.0 0 (Utilities|Array|Get(acopy) (Variables|Attacks|GetAttackCubesIntervals) 2) 0))

(fn SetMeshNormal
  (Components|StaticMesh|SetStaticMesh (Variables|Default|GetStaticMesh) "/Game/Meshes/SM_Teapot_CorrectScale.SM_Teapot_CorrectScale"))

(fn SetMeshCracked
  (Components|StaticMesh|SetStaticMesh (Variables|Default|GetStaticMesh) "/Game/Meshes/SM_TeapotCracked.SM_TeapotCracked"))

(fn SpawnVulnDamageCollision
  (bind _arrow4 (Variables|Default|GetArrow4))
  (bind _returnvalue (Game|SpawnActorfromClass "/Game/Boss/BP_VulnTrigger.BP_VulnTrigger_C" (Transformation|GetWorldTransform _arrow4) "Undefined" "MultiplyWithRoot" 0 self 0))
  (Transformation|AttachComponentToComponent _returnvalue _arrow4 "None" "KeepWorld" "KeepWorld" "KeepWorld" true))

(fn AttackFlood
  (bind _floodspawnarena (Variables|Default|GetFloodSpawnArena))
  (bind _flooding_duration (Variables|TeaFlood|GetFlooding%20Duration))
  (bind _stay_duration (Variables|TeaFlood|GetStay%20Duration))
  (bind _warning_duration (Variables|TeaFlood|GetWarning%20Duration))
  (bind _returnvalue (Transformation|GetActorLocation _floodspawnarena))
  (Game|SpawnActorfromClass "/Game/JansExperimentLab/BP_TeaFlood.BP_TeaFlood_C" (Math|Transform|MakeTransform (Math|Vector|MakeVector (.x _returnvalue) (.y _returnvalue) -0.1) (Transformation|GetActorRotation _floodspawnarena) "1.000000,1.000000,1.000000") "Undefined" "MultiplyWithRoot" 0 _flooding_duration _stay_duration _warning_duration (Variables|TeaFlood|GetFlood%20Height) 0)
  (return (+ (* _flooding_duration 2.0) (+ _warning_duration _stay_duration))))

(fn FinishAttackExecute2
  (Default|CallAttackDoneP2)
  (Math|Integer|IncrementInt (Variables|Attacks|GetAttacksAmount)
    (:%20%20
      (if (>= (Variables|Attacks|GetAttacksAmount) (Variables|Attacks|GetAttacksToSwichP2))
        (Variables|Attacks|SetAttacksAmount 0)
        (Default|SetStateMoving (Variables|Default|GetAs%20BP%20Boss%20Phase%201Controller))))))