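; BP_Boss_Dummy is a damageable boss dummy that displays its health on an attached widget.
; On BeginPlay it creates a WBP_healthBar, assigns it to the Widget component and sets the initial values.
; The Damage event subtracts the incoming amount from Health and refreshes the bar, with no clamping or death handling.
; Tick rotates the widget toward the player camera, billboard style.
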(event EventBeginPlay
  (bind _returnvalue (UserInterface|CreateWidget "/Game/HUD/WBP_healthBar.WBP_healthBar_C"))
  (bind _output_get (Variables|Default|SetWigetRef _returnvalue))
  (UserInterface|SetWidget (Variables|Default|GetWidget) _output_get)
  (Default|UpdateHealth _output_get (Variables|Default|GetHealth) (Variables|Default|GetMaxHealth)))

(event Collision|EventActorBeginOverlap
  (params (OtherActor :type Actor%20Object%20Reference))
  (|CallParentFunction OtherActor) ; This node is disabled and will not be called.\nDrag off pins to build functionality.
)

(event EventTick
  (params (DeltaSeconds :type Float%20%28single-precision%29))
  (bind _widget (Variables|Default|GetWidget))
  (Transformation|SetWorldRotation _widget (Math|Rotator|FindLookatRotation (Transformation|GetWorldLocation _widget) (Transformation|GetWorldLocation (Variables|/Script/Engine.Actor|GetRootComponent (Game|GetPlayerCameraManager 0)))) false false))

(event EventDamage
  (params (DamageAmount :type Float%20%28double-precision%29))
  (Variables|Default|SetHealth (- (Variables|Default|GetHealth) DamageAmount))
  (Default|UpdateHealth (Variables|Default|GetWigetRef) (Variables|Default|GetHealth) (Variables|Default|GetMaxHealth)))

(fn ConstructionScript
  (|CallParentFunction))