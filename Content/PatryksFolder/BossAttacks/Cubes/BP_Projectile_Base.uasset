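; Base boss-attack cube projectile that chases the player, deals CubeDamage on overlap and destroys itself.
; BeginPlay targets the player, then after an AttackBreak delay sets a fixed speed, adds spinning movement and starts a ten-second lifetime.
; Tick re-aims velocity at the target every frame, independently of the optional homing configured in the construction script.
; A Damage event also destroys the cube.
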(event OnComponentBeginOverlap(BoxCollision)
  (params (OverlappedComponent :type Primitive%20Component%20Object%20Reference) (OtherActor :type Actor%20Object%20Reference) (OtherComp :type Primitive%20Component%20Object%20Reference) (OtherBodyIndex :type Integer) (bFromSweep :type Boolean) (SweepResult :type Hit%20Result%20Structure%20%28by%20ref%29))
  (bind _asbp_third_person_character (Utilities|Casting|CastToBP_ThirdPersonCharacter (Game|GetPlayerCharacter 0)))
  (if (== OtherActor _asbp_third_person_character)
    (Default|DamagePlayer _asbp_third_person_character (Variables|Default|GetCubeDamage))
    (Actor|DestroyActor)))

(event Custom|RotateToTarget
  (Variables|/Script/Engine.MovementComponent|SetVelocity (Variables|Default|GetProjectileMovement) (* (Math|Vector|GetUnitDirection(Vector) (Transformation|GetActorLocation) (Transformation|GetActorLocation (Variables|Target|GetTarget))) (Variables|ProjectileSettings|GetSpeed))))

(event Custom|DestroyCube
  (Actor|DestroyActor))

(event EventBeginPlay
  (bind _asbp_third_person_character (Utilities|Casting|CastToBP_ThirdPersonCharacter (Game|GetPlayerCharacter 0)))
  (Variables|Target|SetTarget _asbp_third_person_character)
  (Variables|Target|GetTarget
    (:then
      (Utilities|FlowControl|Delay (Variables|Default|GetAttackBreak))
      (Variables|ProjectileSettings|SetSpeed 5e+02)
      (CallFunction|RotatetoTarget)
      (AddComponent|AddRotatingMovementComponent)
      (Utilities|Time|SetTimerbyEvent (delegate Custom|DestroyCube) 1e+01))
    (:else)))

(event EventDamage
  (params (DamageAmount :type Float%20%28double-precision%29))
  (Actor|DestroyActor))

(event EventTick
  (params (DeltaSeconds :type Float%20%28single-precision%29))
  (CallFunction|RotatetoTarget))

(fn ConstructionScript
  (bind _projectilemovement (Variables|Default|GetProjectileMovement))
  (Variables|/Script/Engine.ProjectileMovementComponent|SetInitialSpeed _projectilemovement (Variables|ProjectileSettings|GetSpeed))
  (Variables|/Script/Engine.ProjectileMovementComponent|SetMaxSpeed _projectilemovement (Variables|ProjectileSettings|GetSpeed))
  (Variables|/Script/Engine.ProjectileMovementComponent|SetProjectileGravityScale _projectilemovement (Variables|ProjectileSettings|GetGravity))
  (Variables|Default|SetAttackBreak (Variables|Default|GetAttackBreak))
  (Variables|Target|GetTarget
    (:then
      (if (Variables|Default|GetIsHoming)
        (Variables|/Script/Engine.ProjectileMovementComponent|SetbIsHomingProjectile _projectilemovement true)
        (Variables|/Script/Engine.ProjectileMovementComponent|SetHomingTargetComponent _projectilemovement (Variables|/Script/Engine.Actor|GetRootComponent (Variables|Target|GetTarget)))))
    (:else)))