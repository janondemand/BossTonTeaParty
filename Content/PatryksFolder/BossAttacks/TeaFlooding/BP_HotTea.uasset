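; BP_HotTea is a boss tea-flooding hazard that burns the player while they stand in it and destroys itself after 30 seconds.
; When the player character enters its Box, a looping timer starts and calls DamagePlayer with FloorDamage every tenth of a second.
; Leaving the Box clears that timer, so damage stops.
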(event OnComponentEndOverlap(Box)
  (params (OverlappedComponent :type Primitive%20Component%20Object%20Reference) (OtherActor :type Actor%20Object%20Reference) (OtherComp :type Primitive%20Component%20Object%20Reference) (OtherBodyIndex :type Integer))
  (bind _asbp_third_person_character (Utilities|Casting|CastToBP_ThirdPersonCharacter (Game|GetPlayerCharacter 0)))
  (if (== OtherActor _asbp_third_person_character)
    (Utilities|Time|ClearandInvalidateTimerbyHandle (Variables|Default|GetTimer))))

(event OnComponentBeginOverlap(Box)
  (params (OverlappedComponent :type Primitive%20Component%20Object%20Reference) (OtherActor :type Actor%20Object%20Reference) (OtherComp :type Primitive%20Component%20Object%20Reference) (OtherBodyIndex :type Integer) (bFromSweep :type Boolean) (SweepResult :type Hit%20Result%20Structure%20%28by%20ref%29))
  (bind _asbp_third_person_character (Utilities|Casting|CastToBP_ThirdPersonCharacter (Game|GetPlayerCharacter 0)))
  (if (== OtherActor _asbp_third_person_character)
    (bind _returnvalue (Utilities|Time|SetTimerbyEvent (delegate Custom|HotTeaDamage) 0.1 true))
    (Variables|Default|SetTimer _returnvalue)))

(event Custom|HotTeaDamage
  (Default|DamagePlayer (stale OnComponentBeginOverlap(Box) _asbp_third_person_character) (Variables|Default|GetFloorDamage)))

(event EventBeginPlay
  (Utilities|FlowControl|Delay 3e+01)
  (Actor|DestroyActor))

(fn ConstructionScript)